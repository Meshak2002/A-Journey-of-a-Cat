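; BP_Parallax is an image actor that fakes parallax by tilting in response to the player's camera.
; The construction script creates a dynamic material on the Image component and sets its BackgroundImage texture.
; BeginPlay caches the BP_Suraa player character.
; Each Tick smoothly interpolates rotation toward the camera-to-actor look-at direction, clamping pitch and yaw to narrow ranges and preserving roll.
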(event EventBeginPlay
  (bind _asbp_suraa (Utilities|Casting|CastToBP_Suraa (Game|GetPlayerCharacter 0)))
  (Utilities|IsValid _asbp_suraa
    (:Is%20Valid
      (Variables|Default|SetAs%20BP%20Suraa _asbp_suraa))))

(event Collision|EventActorBeginOverlap
  (params (OtherActor :type Actor%20Object%20Reference)))

(event EventTick
  (params (DeltaSeconds :type Float%20%28single-precision%29))
  (bind _returnvalue (Transformation|GetActorLocation))
  (bind _returnvalue_2 (Transformation|GetActorRotation))
  (bind _as_bp_suraa (Variables|Default|GetAs%20BP%20Suraa))
  (bind _camera (Variables|/Game/TheJourneyDennis/BP_Suraa.BP_Suraa_C|GetCamera _as_bp_suraa))
  (bind _returnvalue_3 (Transformation|GetWorldLocation _camera))
  (bind _returnvalue_4 (Math|Rotator|FindLookatRotation _returnvalue_3 _returnvalue))
  (bind _returnvalue_5 (Math|Interpolation|RInterpTo _returnvalue_2 _returnvalue_4 DeltaSeconds 1e+01))
  (bind (_roll _pitch _yaw) (Math|Rotator|BreakRotator _returnvalue_5))
  (Transformation|SetActorRotation (Math|Rotator|MakeRotator (.Roll (Math|Rotator|BreakRotator _returnvalue_2)) (Math|Float|ClampAngle _pitch -1e+01 1e+01) (Math|Float|ClampAngle _yaw -3e+01 3e+01))))

(fn ConstructionScript
  (bind _returnvalue (Rendering|Material|CreateDynamicMaterialInstance (Variables|Default|GetImage) 0 0 "None" :!class /Script/Engine.PrimitiveComponent))
  (Rendering|Material|SetTextureParameterValue _returnvalue "BackgroundImage" (Variables|BGimage|GetValue)))