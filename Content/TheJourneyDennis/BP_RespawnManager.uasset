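; BP_RespawnManager is a checkpoint tracker that updates the spawn point of the BP_Sora player as they advance along world Y.
; BeginPlay caches the player, then Tick scans the RespawnPoint array, converting actor-relative locations to world space.
; Each point the player's Y exceeds becomes SpawnPoint, with X pinned to a hardcoded value.
; The saved index starts later scans, so earlier checkpoints are never revisited.
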(event EventBeginPlay
  (bind _asbp_sora (Utilities|Casting|CastToBP_Sora (Game|GetPlayerCharacter 0)))
  (Variables|Default|SetAs%20BP%20Sora _asbp_sora)
  (Variables|Default|SetItr 0))

(event EventTick
  (params (DeltaSeconds :type Float%20%28single-precision%29))
  (bind _returnvalue (Transformation|GetActorTransform))
  (for _index (range (Variables|Default|GetItr) (- (Utilities|Array|Length (Variables|Default|GetRespawnPoint)) 1))
    (if (> (.y (Transformation|GetActorLocation (Variables|Default|GetAs%20BP%20Sora))) (.y (Math|Transform|TransformLocation _returnvalue (.location (Utilities|Array|Get(acopy) (Variables|Default|GetRespawnPoint) _index)))))
      (Variables|Default|SetCurrentSpawnPoint (Math|Transform|MakeTransform (Math|Transform|TransformLocation _returnvalue (.location (Utilities|Array|Get(acopy) (Variables|Default|GetRespawnPoint) _index))) "0, 0, 0" "1.000000,1.000000,1.000000"))
      (Variables|/Game/TheJourney/BP_Sora.BP_Sora_C|SetSpawnPoint (Variables|Default|GetAs%20BP%20Sora) (Math|Transform|MakeTransform (Math|Vector|MakeVector 1956.847644 (.y (.location (Variables|Default|GetCurrentSpawnPoint))) (.z (.location (Variables|Default|GetCurrentSpawnPoint)))) "0, 0, 0" "1.000000,1.000000,1.000000"))
      (Variables|Default|SetItr _index))))

(fn ConstructionScript)